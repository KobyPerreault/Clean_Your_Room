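; Spawner actor that creates NegativeObject_BP instances at random points inside a box volume.
; On BeginPlay it binds its Spawn event to the RespawnNegativeObject dispatcher on FirstPersonGameMode, so spawning happens only when that event fires.
; Each spawned object is added to the SpawnActor array.
; The construction script sizes SpawnVolume from the BoxExtent variable, which also bounds the random spawn location.
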(event Custom|Spawn
  (bind _returnvalue (Game|SpawnActorfromClass "/Game/Room_BPs/NegativeObject_BP.NegativeObject_BP_C" (Math|Transform|MakeTransform (Math|Random|RandomPointinBoundingBox (Transformation|GetWorldLocation (Variables|Default|GetSpawnVolume)) (Variables|Default|GetBoxExtent)) "0, 0, 0" "1,1,1") "Undefined" 0 0))
  (Utilities|Array|Add (Variables|Default|GetSpawn%20Actor) _returnvalue))

(event EventBeginPlay
  (bind _asfirst_person_game_mode (Utilities|Casting|CastToFirstPersonGameMode (Game|GetGameMode)))
  (EventDispatchers|BindEventtoRespawnNegativeObject _asfirst_person_game_mode (delegate Custom|Spawn)))

(fn ConstructionScript
  (Components|Box|SetBoxExtent (Variables|Default|GetSpawnVolume) (Variables|Default|GetBoxExtent) true))